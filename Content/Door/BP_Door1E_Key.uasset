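; BP_Door1E_Key is a key-locked door that the player toggles open and closed with the OpenDoor input.
; Its Box overlap stores the third-person character, enables input and opens a gate, both shut off again on exit.
; With the character's HasKey set, a FlipFlop plays or reverses a timeline that lerps door yaw between closed and open angles.
; Without the key, it plays a sound at the door.
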(event OnComponentBeginOverlap(Box)
  (params (OverlappedComponent :type Primitive%20Component%20Object%20Reference) (OtherActor :type Actor%20Object%20Reference) (OtherComp :type Primitive%20Component%20Object%20Reference) (OtherBodyIndex :type Integer) (bFromSweep :type Boolean) (SweepResult :type Hit%20Result%20Structure%20%28by%20ref%29))
  (bind _asbp_third_person_character (Utilities|Casting|CastToBP_ThirdPersonCharacter OtherActor))
  (Input|EnableInput (Game|GetPlayerController 0))
  (Utilities|FlowControl|Gate true) ; enters at Open
)

(event OnComponentEndOverlap(Box)
  (params (OverlappedComponent :type Primitive%20Component%20Object%20Reference) (OtherActor :type Actor%20Object%20Reference) (OtherComp :type Primitive%20Component%20Object%20Reference) (OtherBodyIndex :type Integer))
  (Utilities|Casting|CastToBP_ThirdPersonCharacter OtherActor)
  (Input|DisableInput (Game|GetPlayerController 0))
  (Utilities|FlowControl|Gate true) ; enters at Close
)

(event EventBeginPlay)

(event Collision|EventActorBeginOverlap
  (params (OtherActor :type Actor%20Object%20Reference)))

(event EventTick
  (params (DeltaSeconds :type Float%20%28single-precision%29)))

(event Input|ActionEvents|InputActionOpenDoor
  (params (Key :type Key%20Structure :default "None"))
  (:Pressed
    (if (Variables|/Game/ThirdPerson/Blueprints/BP_ThirdPersonCharacter.BP_ThirdPersonCharacter_C|GetHas%20Key? (stale OnComponentBeginOverlap(Box) _asbp_third_person_character))
      (Utilities|FlowControl|Gate true
        (:Exit
          (Utilities|FlowControl|FlipFlop
            (:A
              (bind _alpha (Timeline|Open/Close Play)
                (:Update
                  (Transformation|SetRelativeRotation (Variables|Default|GetDoor) (Math|Rotator|MakeRotator 0.0 0.0 (Math|Float|Lerp (Variables|Default|GetClose%20Angle) (Variables|Default|GetOpen%20Angle) _alpha)) false false))))
            (:B
              (Timeline|Open/Close Reverse)))))
      (else
        (Audio|PlaySoundatLocation 0 (Transformation|GetActorLocation) "0, 0, 0" 1.0 1.0 0.0 0 0 0 0)))))

(fn ConstructionScript)